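; BP_HMI is a training-system actor that presents a description widget (WBP_HMI_WidgetComponent) through a widget component alongside a box collision.
; Begin Play caches the widget, and helper functions set its description text and toggle its visibility.
; Construction resets the actor's tags to IDTag and grows the box's X/Y extent by DistanceOffset.
; Box visibility follows the Debug flag on activation toggles, or at construction when AutoActivate is set.
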(event EventBeginPlay
  ;[0 1 0] Begin Play
  (|CallParentFunction)
  (bind _aswbp_hmi_widget_component (Utilities|Casting|CastToWBP_HMI_WidgetComponent (UserInterface|GetUserWidgetObject (Variables|Default|GetHMI_Widget))))
  (Variables|Default|SetWBP%20HMI%20Widget%20Component _aswbp_hmi_widget_component))

(event EventToggleActorActive
  (params (bActivate :type Boolean))
  (|CallParentFunction bActivate)
  (Development|SetHiddeninGame (Variables|Default|GetBoxCollision) (not (Variables|Settings|GetbDebug)) false))

(fn ConstructionScript
  (bind _tags (Variables|Default|GetTags))
  (bind _boxcollision (Variables|Default|GetBoxCollision))
  (bind _distanceoffset (Variables|Settings|GetDistanceOffset))
  (bind (_x _y) (Math|Vector2D|BreakVector2D _distanceoffset))
  (|CallParentFunction)
  (Utilities|Array|Clear _tags)
  (Utilities|Array|Add _tags (Variables|Settings|GetID_Tag))
  (Components|Box|SetBoxExtent _boxcollision (+ (Variables|/Script/Engine.BoxComponent|GetBoxExtent _boxcollision) (Math|Vector|MakeVector _x _y 0.0)) true)
  (if (Variables|Default|GetbAutoActivate)
    (Development|SetHiddeninGame (Variables|Default|GetBoxCollision) (not (Variables|Settings|GetbDebug)) false)))

(fn SetHMIWidgetText
  (params (InText :type Text))
  (Default|SetDescriptionText (Variables|Default|GetWBP%20HMI%20Widget%20Component) InText))

(fn ToggleHMIWidgetVisibility
  (params (bVisibility :type Boolean))
  (Rendering|SetVisibility (Variables|Default|GetHMI_Widget) bVisibility false))