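; BP_ActivationActor is an actor in the training management system that can be switched fully on or off.
; The ToggleActorActive event drives visibility, tick and collision together from a single Activate flag.
; The construction script applies the same three settings from AutoActivate, which sets the actor's initial state.
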(event Custom|ToggleActorActive
  (params (bActivate :type Boolean))
  (Rendering|SetActorHiddenInGame (not bActivate))
  (Actor|Tick|SetActorTickEnabled bActivate)
  (Collision|SetActorEnableCollision bActivate))

(fn ConstructionScript
  (bind _bautoactivate (Variables|Settings|GetbAutoActivate))
  (Rendering|SetActorHiddenInGame (not (Variables|Settings|GetbAutoActivate)))
  (Actor|Tick|SetActorTickEnabled _bautoactivate)
  (Collision|SetActorEnableCollision _bautoactivate))