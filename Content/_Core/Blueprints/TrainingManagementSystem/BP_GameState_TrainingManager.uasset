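; Game state that manages a training sequence of BP_HMI steps, loading step data from a data table into a map keyed by ID tag.
; On BeginPlay it sets HMI texts and builds the HUD checklist.
; Completion attempts route through server and all events to tick the checklist, update HMI text, toggle tagged activation actors and check whether all steps are done.
; A debug option auto-completes steps preceding a chosen tag.
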(event Custom|AttemptComplete_All
  (params (InCurrentBP_HMI :type BP%20HMI%20Object%20Reference))
  ;[1 1 1] Attempt Completion
  (CallFunction|SetTrainingStepComplete (Variables|/Game/_Core/Blueprints/TrainingManagementSystem/BP_HMI.BP_HMI_C|GetID_Tag InCurrentBP_HMI))
  (CallFunction|ToggleActivationActors (Variables|/Game/_Core/Blueprints/TrainingManagementSystem/BP_HMI.BP_HMI_C|GetActorsToActivateOnInteract InCurrentBP_HMI) true)
  (CallFunction|ToggleActivationActors (Variables|/Game/_Core/Blueprints/TrainingManagementSystem/BP_HMI.BP_HMI_C|GetActorsToDeactivateOnInteract InCurrentBP_HMI) false)
  (bind _btrainingcompleted (CallFunction|CheckifAllTrainingCompleted))
  (if _btrainingcompleted
    (Development|PrintString "Game Over")))

(event Custom|AttemptComplete_Server
  (params (InCurrentBP_HMI :type BP%20HMI%20Object%20Reference))
  ;[1 1 1] Attempt Completion
  (CallFunction|AttemptCompleteAll InCurrentBP_HMI))

(event EventBeginPlay
  ;[0 1 0] Begin Play
  (Utilities|FlowControl|Sequence
    (:then_0
      (bind _outactors (Actor|GetAllActorsOfClass "/Game/_Core/Blueprints/TrainingManagementSystem/BP_HMI.BP_HMI_C"))
      (Variables|Default|SetBP_HMI_Array _outactors))
    (:then_1
      (CallFunction|InitTrainingManagementData))
    (:then_2
      (CallFunction|InitBPHMIArraywithTrainingManagementData))
    (:then_3
      ;;[1 1 1] Delay to allow the HUD to generate the overlay widget
      (Utilities|FlowControl|Delay 0.2)
      (bind _returnvalue (Actor|GetActorOfClass "/Game/_Core/Blueprints/BP_HUD.BP_HUD_C"))
      (Variables|Default|SetWBP%20HUD%20Overlay (Variables|/Game/_Core/Blueprints/BP_HUD.BP_HUD_C|GetWBP_HUD_Overlay _returnvalue))
      (CallFunction|InitTrainingChecklist))
    (:then_4
      ;;[1 1 1] Debug Game If Necessary. Set bDebug True and DebugTrainingID_Tag to jump to the training step you wish to debug.
      (Utilities|FlowControl|Delay 1.0)
      (CallFunction|DebugJumptoTrainingStep))))

(event EventAttemptHMIComplete
  (params (InCurrentBP_HMI :type BP%20HMI%20Object%20Reference))
  ;[1 1 1] Attempt Completion
  (CallFunction|AttemptCompleteServer InCurrentBP_HMI))

(fn ConstructionScript)

(fn InitTrainingManagementData
  (bind _datatablefortraining (Variables|Default|GetDataTableForTraining))
  (Utilities|Map|Clear (Variables|Default|GetTrainingDataMap))
  (bind _outrownames (DataTable|GetDataTableRowNames _datatablefortraining))
  (for _array_element _outrownames
    (bind _returnvalue (Utilities|GetDataTableRow _datatablefortraining _array_element)
      (:then
        (Utilities|Map|Add (Variables|Default|GetTrainingDataMap) (.ID_Tag (Utilities|Struct|BreakTrainingManagement_Struct _returnvalue)) _returnvalue))))
  (return))

(fn InitBPHMIArraywithTrainingManagementData
  (for _array_element (Variables|Default|GetBP_HMI_Array)
    (if (.ReturnValue (Utilities|Map|Find (Variables|Default|GetTrainingDataMap) (Variables|/Game/_Core/Blueprints/TrainingManagementSystem/BP_HMI.BP_HMI_C|GetID_Tag _array_element)))
      (Default|SetHMIWidgetText _array_element (Utilities|Text|ToText(String) (.HMI_NotStartedText (Utilities|Struct|BreakTrainingManagement_Struct (.Value (Utilities|Map|Find (Variables|Default|GetTrainingDataMap) (Variables|/Game/_Core/Blueprints/TrainingManagementSystem/BP_HMI.BP_HMI_C|GetID_Tag _array_element))))))))))

(fn InitTrainingChecklist
  (bind _wbp_hud_overlay (Variables|Default|GetWBP%20HUD%20Overlay)
    (:then
      (Default|InitTrainingChecklistScrollBox (Variables|/Game/_Core/UI/WBP_HUD_Overlay.WBP_HUD_Overlay_C|GetTrainingChecklist _wbp_hud_overlay)))
    (:else)))

(fn SetTrainingStepComplete
  (params (InCurrentID_Tag :type Name))
  ;[1 1 1] Set the checklist as checked for this training step
  (bind _array_element (Utilities|Array|ForEachLoopwithBreak (Class|PanelWidget|GetAllChildren (Variables|/Game/_Core/UI/TrainingChecklist/WBP_TrainingChecklist.WBP_TrainingChecklist_C|GetTrainingChecklistScrollbox (Variables|/Game/_Core/UI/WBP_HUD_Overlay.WBP_HUD_Overlay_C|GetTrainingChecklist (Variables|Default|GetWBP%20HUD%20Overlay)))) :!label _label)
    (:LoopBody
      (bind _aswbp_checklist_button (Utilities|Casting|CastToWBP_ChecklistButton _array_element))
      (if (== (Variables|/Game/_Core/UI/TrainingChecklist/Components/WBP_ChecklistButton.WBP_ChecklistButton_C|GetID_Tag _aswbp_checklist_button) InCurrentID_Tag)
        (Default|ToggleCheckboxState _aswbp_checklist_button true)
        (goto _label Break)))
    (:Completed
      ;[1 1 1] Set the training management data for this training step as completed
      (bind _structout (Utilities|Struct|SetmembersinTrainingManagement_Struct (.Value (Utilities|Map|Find (Variables|Default|GetTrainingDataMap) InCurrentID_Tag)) true))
      (Utilities|Map|Add (Variables|Default|GetTrainingDataMap) InCurrentID_Tag _structout)
      ;[1 1 1] Set the HMI Text as 'completed"
      (bind _currentbp_hmi (CallFunction|GetCurrentBPHMIfromID InCurrentID_Tag))
      (Default|SetHMIWidgetText _currentbp_hmi (Utilities|Text|ToText(String) (Utilities|Struct|BreakTrainingManagement_Struct (.Value (Utilities|Map|Find (Variables|Default|GetTrainingDataMap) InCurrentID_Tag))))))))

(fn CheckifAllTrainingCompleted
  (LocalVariables|SetlocalTrainingCompleted true)
  (bind _values (Utilities|Map|Values (Variables|Default|GetTrainingDataMap)))
  (bind _array_element (Utilities|Array|ForEachLoopwithBreak _values :!label _label)
    (:LoopBody
      ;[1 1 1] If we find one HMI not completed, then the entire training is not complete.
      (if (not (.bCompleted (Utilities|Struct|BreakTrainingManagement_Struct _array_element)))
        (LocalVariables|SetlocalTrainingCompleted false)
        (goto _label Break)))
    (:Completed
      (return (LocalVariables|GetlocalTrainingCompleted)))))

(fn ToggleActivationActors
  (params (ActivationActors :type Array%20of%20Names) (bActivate :type Boolean))
  (if (Utilities|Array|IsValidIndex ActivationActors)
    (for _array_element ActivationActors
      (bind _outactors (Actor|GetAllActorsOfClasswithTag "/Game/_Core/Blueprints/TrainingManagementSystem/BP_ActivationActor.BP_ActivationActor_C" _array_element))
      (for _array_element_2 _outactors
        (Default|ToggleActorActive _array_element_2 bActivate))))
  (return))

(fn DebugJumptoTrainingStep
  (if (Variables|Debug|GetbDebug)
    (bind _values (Utilities|Map|Values (Variables|Default|GetTrainingDataMap)))
    (bind _array_element (Utilities|Array|ForEachLoopwithBreak _values :!label _label)
      (:LoopBody
        (if (== (.ID_Tag (Utilities|Struct|BreakTrainingManagement_Struct _array_element)) (Variables|Debug|GetDebugTrainingID_Tag))
          (goto _label Break)
          (else
            (bind _currentbp_hmi (CallFunction|GetCurrentBPHMIfromID (.ID_Tag (Utilities|Struct|BreakTrainingManagement_Struct _array_element))))
            (CallFunction|AttemptHMIComplete _currentbp_hmi)
            (CallFunction|SetTrainingStepComplete (.ID_Tag (Utilities|Struct|BreakTrainingManagement_Struct _array_element)))))))))

(fn GetCurrentBPHMIfromID
  (params (InCurrentID_Tag :type Name :default "None"))
  (bind _array_element (Utilities|Array|ForEachLoopwithBreak (Variables|Default|GetBP_HMI_Array) :!label _label)
    (:LoopBody
      (if (== (Variables|/Game/_Core/Blueprints/TrainingManagementSystem/BP_HMI.BP_HMI_C|GetID_Tag _array_element) InCurrentID_Tag)
        (LocalVariables|SetlocalCurrentBP_HMI _array_element)
        (goto _label Break)))
    (:Completed
      (return (LocalVariables|GetlocalCurrentBP_HMI)))))

(fn GetCurrentTrainingStepDatafromID
  (params (InCurrentID_Tag :type Name :default "None"))
  (return (.Value (Utilities|Map|Find (Variables|Default|GetTrainingDataMap) InCurrentID_Tag))))

(fn GetTrainingDataMap
  (return (Variables|Default|GetTrainingDataMap)))

(fn GetWBPHUDOverlay
  (return (Variables|Default|GetWBP%20HUD%20Overlay)))