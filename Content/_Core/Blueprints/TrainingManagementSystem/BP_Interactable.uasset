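; BP_Interactable is an interactable object in the training management system, with a box collision for interaction.
; Its construction script replaces all existing Tags with a single IDTag, which identifies the object.
; It also enlarges the InteractionCollision box horizontally by adding the X and Y of DistanceOffset to its extent, leaving the height unchanged.
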(fn ConstructionScript
  (bind _tags (Variables|Actor|GetTags))
  (bind _interactioncollision (Variables|Default|GetInteractionCollision))
  (bind _distanceoffset (Variables|Settings|GetDistanceOffset))
  (bind (_x _y) (Math|Vector2D|BreakVector2D _distanceoffset))
  (Utilities|Array|Clear _tags)
  (Utilities|Array|Add _tags (Variables|Settings|GetID_Tag))
  (Components|Box|SetBoxExtent _interactioncollision (+ (Variables|/Script/Engine.BoxComponent|GetBoxExtent _interactioncollision) (Math|Vector|MakeVector _x _y 0.0)) true))